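; BP_NeonVehicle is a vehicle Blueprint that plays 2D sound cues for player-controlled movement and power-up changes.
; Each Tick compares airborne state, a thresholded steering state, active power-up type and held power-up against cached values, firing sounds only on changes.
; Movement transitions trigger takeoff, landing and turn sounds, while power-up changes trigger pickup and type-specific activation sounds.
; The graph contains only this audio logic, reading state from the Movement and Powerups objects.
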(event `self.ReceiveTick`
  (params (DeltaSeconds :type "Float (single-precision)"))
  (bind _returnvalue (`NeonPowerupComponent.GetActiveType` (`self.Powerups`)))
  (bind _returnvalue_2 (`NeonPowerupComponent.GetHeld` (`self.Powerups`)))
  (bind _returnvalue_3 (`NeonMovementComponent.IsAirborne` (`self.Movement`)))
  (bind _returnvalue_4 (> (`KismetMathLibrary.Abs` (`NeonMovementComponent.GetAppliedSteering` (`self.Movement`))) 0.6))
  (if (`self.IsPlayerControlled`)
    (`|ExecutionSequence`
      (:`then_0`
        (if (!= _returnvalue_3 (`self.bWasAir`))
          (set `self.bWasAir` _returnvalue_3)
          (if _returnvalue_3
            (`GameplayStatics.PlaySound2D` "/Game/NwiroAssets/Audio/sfx/Futuristic_motorcycle_jump_takeoff_engin.Futuristic_motorcycle_jump_takeoff_engin" 1.0 1.0 0.0 null null)
            (else
              (`GameplayStatics.PlaySound2D` "/Game/NwiroAssets/Audio/sfx/Heavy_sci_fi_motorcycle_landing_on_hard_.Heavy_sci_fi_motorcycle_landing_on_hard_" 1.0 1.0 0.0 null null)))))
      (:`then_1`
        (`|ExecutionSequence`
          (:`then_0`
            (if (!= _returnvalue_4 (`self.bWasTurning`))
              (set `self.bWasTurning` _returnvalue_4)
              (if _returnvalue_4
                (`GameplayStatics.PlaySound2D` "/Game/NwiroAssets/Audio/sfx/sharp_light_cycle_90_degree_turn_quick_e.sharp_light_cycle_90_degree_turn_quick_e" 0.7 1.0 0.0 null null)
                (else
                  (`GameplayStatics.PlaySound2D` "/Game/NwiroAssets/Audio/sfx/Light_cycle_weaving_side_to_side_quick_s.Light_cycle_weaving_side_to_side_quick_s" 0.4 1.0 0.0 null null)))))
          (:`then_1`
            (`|ExecutionSequence`
              (:`then_0`
                (if (!= _returnvalue (`self.LastActive`))
                  (set `self.LastActive` _returnvalue)
                  (`|ExecutionSequence`
                    (:`then_0`
                      (if (== _returnvalue 3)
                        (`GameplayStatics.PlaySound2D` "/Game/NwiroAssets/Audio/sfx/Phase_shift_activate_ghostly_digital_war.Phase_shift_activate_ghostly_digital_war" 1.0 1.0 0.0 null null)
                        (elif (== _returnvalue 4)
                          (`GameplayStatics.PlaySound2D` "/Game/NwiroAssets/Audio/sfx/Laser_trail_cutter_sharp_energy_blade_sl.Laser_trail_cutter_sharp_energy_blade_sl" 1.0 1.0 0.0 null null))))
                    (:`then_1`
                      (`|ExecutionSequence`
                        (:`then_0`
                          (if (== _returnvalue 5)
                            (`GameplayStatics.PlaySound2D` "/Game/NwiroAssets/Audio/sfx/EMP_blast_electromagnetic_pulse_shockwav.EMP_blast_electromagnetic_pulse_shockwav" 1.0 1.0 0.0 null null)
                            (elif (== _returnvalue 6)
                              (`GameplayStatics.PlaySound2D` "/Game/NwiroAssets/Audio/sfx/Overdrive_activate_powerful_synth_engine.Overdrive_activate_powerful_synth_engine" 1.0 1.0 0.0 null null)))))))))
              (:`then_1`
                (if (!= _returnvalue_2 (`self.LastHeld`))
                  (set `self.LastHeld` _returnvalue_2)
                  (if (!= _returnvalue_2 0)
                    (`GameplayStatics.PlaySound2D` "/Game/NwiroAssets/Audio/sfx/Power_up_pickup_sparkling_futuristic_chi.Power_up_pickup_sparkling_futuristic_chi" 1.0 1.0 0.0 null null)))))))))))

(fn `UserConstructionScript`)