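; Neon arena actor that restyles its Terrain component with the M_TronGrid material.
; Every Tick it checks whether the first material slot is based on BasicShapeMaterial.
; If so, it swaps each slot for a dynamic M_TronGrid instance, copying over the Color parameter from the existing dynamic instance.
; Polling lets it catch materials assigned after spawn; the base-material check skips terrain already converted.
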(event `self.ReceiveTick`
  (params (DeltaSeconds :type "Float (single-precision)"))
  (bind _terrain (`self.Terrain`))
  (bind _returnvalue (`PrimitiveComponent.GetMaterial` _terrain 0))
  (if (`KismetSystemLibrary.IsValid` _returnvalue)
    (bind _returnvalue_2 (`MaterialInterface.GetBaseMaterial` _returnvalue))
    (if (== _returnvalue_2 "/Engine/BasicShapes/BasicShapeMaterial.BasicShapeMaterial")
      (for _index (range (`PrimitiveComponent.GetNumMaterials` _terrain))
        (bind _asmaterial_instance_dynamic (cast `MaterialInstanceDynamic` (`PrimitiveComponent.GetMaterial` _terrain _index)))
        (bind _returnvalue_3 (`MaterialInstanceDynamic.K2_GetVectorParameterValue` _asmaterial_instance_dynamic "Color"))
        (bind _returnvalue_4 (`PrimitiveComponent.CreateDynamicMaterialInstance` _terrain _index "/Game/NeonGrid/Materials/M_TronGrid.M_TronGrid" "None"))
        (`MaterialInstanceDynamic.SetVectorParameterValue` _returnvalue_4 "Color" _returnvalue_3)))))

(fn `UserConstructionScript`)