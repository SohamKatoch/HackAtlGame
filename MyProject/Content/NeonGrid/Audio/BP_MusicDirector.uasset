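; Music director actor that switches music and plays stingers in response to the match phase in NeonGameState.
; It polls the phase every Tick, caching the last values so each change fires only once.
; Menu and battle tracks crossfade when entering or leaving the menu phase.
; Phase changes also trigger a round-end chime, or a match-end victory or defeat sting depending on whether slot 0 won.
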(event `self.ReceiveTick`
  (params (DeltaSeconds :type "Float (single-precision)"))
  (bind _menumusic (`self.MenuMusic`))
  (bind _battlemusic (`self.BattleMusic`))
  (bind _asneon_game_state (cast `NeonGameState` (`GameplayStatics.GetGameState`)))
  (`|ExecutionSequence`
    (:`then_0`
      (bind _returnvalue (`NeonGameState.GetPhase` _asneon_game_state))
      (bind _returnvalue_2 (== _returnvalue 0))
      (if (!= _returnvalue_2 (`self.bWasMenu`))
        (set `self.bWasMenu` _returnvalue_2)
        (if _returnvalue_2
          (`AudioComponent.FadeIn` _menumusic 1.5 1.0 0.0 "Linear")
          (`AudioComponent.FadeOut` _battlemusic 1.5 0.0 "Linear")
          (else
            (`AudioComponent.FadeIn` _battlemusic 1.5 1.0 0.0 "Linear")
            (`AudioComponent.FadeOut` _menumusic 1.5 0.0 "Linear")))))
    (:`then_1`
      (if (!= _returnvalue (`self.LastPhase`))
        (set `self.LastPhase` _returnvalue)
        (`|ExecutionSequence`
          (:`then_0`
            (if (== _returnvalue 3)
              (`GameplayStatics.PlaySound2D` "/Game/NwiroAssets/Audio/sfx/Round_end_chime_futuristic_digital_confi.Round_end_chime_futuristic_digital_confi" 1.0 1.0 0.0 null null)))
          (:`then_1`
            (if (== _returnvalue 4)
              (if (== (`NeonGameState.GetMatchWinnerSlot` _asneon_game_state) 0)
                (`GameplayStatics.PlaySound2D` "/Game/NwiroAssets/Audio/music/Short_triumphant_victory_sting_Tron_Lega.Short_triumphant_victory_sting_Tron_Lega" 1.0 1.0 0.0 null null)
                (else
                  (`GameplayStatics.PlaySound2D` "/Game/NwiroAssets/Audio/music/Short_defeat_sting_Tron_style_descending.Short_defeat_sting_Tron_style_descending" 1.0 1.0 0.0 null null))))))))))

(fn `UserConstructionScript`)